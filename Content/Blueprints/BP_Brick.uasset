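; BP_Brick is a brick actor that handles level progression when the last brick in the level is destroyed.
; On Destroyed, it counts all BP_Brick actors and proceeds only if exactly one is found.
; It then reads LevelNumber from BP_LevelTracker to open the next level, or shows the BP_WinScreen widget after the third level.
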(event EventDestroyed
  (bind _outactors (Actor|GetAllActorsOfClass "BP_Brick_C"))
  (if (== (Utilities|Array|Length _outactors) 1)
    (bind _returnvalue (Actor|GetActorOfClass "/Game/Blueprints/BP_LevelTracker.BP_LevelTracker_C"))
    (switch int (Variables|/Game/Blueprints/BP_LevelTracker.BP_LevelTracker_C|GetLevelNumber _returnvalue)
      (:1
        (Game|OpenLevel(byObjectReference) "/Game/Maps/Level2.Level2"))
      (:2
        (Game|OpenLevel(byObjectReference) "/Game/Maps/Level3.Level3"))
      (:3
        (bind _returnvalue_2 (UserInterface|CreateWidget "/Game/Blueprints/UI/BP_WinScreen.BP_WinScreen_C"))
        (UserInterface|Viewport|AddtoViewport _returnvalue_2 0)))))

(fn ConstructionScript)